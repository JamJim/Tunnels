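; Player controller that fires projectiles from the controlled pawn toward the point under the mouse cursor while a mouse button is held.
; Left and right buttons open separate Tick-driven gates, spawning ProjectileBP and ProjectileBP1 respectively.
; A short Delay after each gate throttles fire rate, then a cursor Visibility trace aims the spawn from an offset above the pawn.
; Logic to turn the pawn toward the cursor is present but unconnected.
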(event `self.ReceiveTick`
  (params (DeltaSeconds :type "Float (single-precision)"))
  (bind _returnvalue (`self.K2_GetActorLocation` (`self.K2_GetPawn`)))
  (bind _returnvalue_2 (`self.K2_GetActorLocation` (`self.K2_GetPawn`)))
  ;[1 1 1] Shoot in direction of mouse
  (`|ExecutionSequence`
    (:`then_0`
      (`/Engine/EditorBlueprintResources/StandardMacros.Gate` true :!label _label
        (:`Exit`
          (`KismetSystemLibrary.Delay` 0.1)
          (`|SpawnActorFromClass` "/Game/ProjectileBP1.ProjectileBP1_C" (`KismetMathLibrary.MakeTransform` (+ _returnvalue (100.0 0.0 200.0)) (`KismetMathLibrary.FindLookAtRotation` _returnvalue (`.Location` (`GameplayStatics.BreakHitResult` (`self.GetHitResultUnderCursorByChannel` "TraceTypeQuery1"))))) "Undefined" "OverrideRootScale" null null))))
    (:`then_1`
      (`/Engine/EditorBlueprintResources/StandardMacros.Gate` true :!label _label_2
        (:`Exit`
          (`KismetSystemLibrary.Delay` 0.1)
          (`|SpawnActorFromClass` "/Game/ProjectileBP.ProjectileBP_C" (`KismetMathLibrary.MakeTransform` (+ _returnvalue_2 (100.0 0.0 200.0)) (`KismetMathLibrary.FindLookAtRotation` _returnvalue_2 (`.Location` (`GameplayStatics.BreakHitResult` (`self.GetHitResultUnderCursorByChannel` "TraceTypeQuery1"))))) "Undefined" "OverrideRootScale" null null))))))

(event `Key|RightMouseButton`
  (params (Key :type "Key Structure"))
  (:`Pressed`
    (goto _label :!via `Open`))
  (:`Released`
    (goto _label :!via `Close`)))

(event `Key|LeftMouseButton`
  (params (Key :type "Key Structure"))
  ;[1 1 1] Shoot in direction of mouse
  (:`Pressed`
    (goto _label_2 :!via `Open`))
  (:`Released`
    (goto _label_2 :!via `Close`)))

(fn `UserConstructionScript`)